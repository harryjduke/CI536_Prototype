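; BP_BreakableDoors is a double door that swings open when a BP_Abomination overlaps it; despite the name, no breaking logic appears here.
; BeginPlay derives mirrored open rotations from each side's closed relative rotation.
; OpenDoors and CloseDoors set a state that Tick uses to interpolate both sides via InterpDoorRotation.
; End-state checks compare world rotation against those relative targets; nothing here calls CloseDoors.
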(event `self.ReceiveBeginPlay`
  ;[1 1 1] Set open and closed rotations
  (bind _output_get (set `self.ClosedRotationLeft` (`SceneComponent.RelativeRotation` (`self.LeftSideDoor`))))
  (set `self.OpenRotationLeft` (`KismetMathLibrary.ComposeRotators` _output_get (`KismetMathLibrary.MakeRotator` 0.0 0.0 (`self.RotateAmount`))))
  (bind _output_get_2 (set `self.ClosedRotationRight` (`SceneComponent.RelativeRotation` (`self.RightSideDoor`))))
  (set `self.OpenRotationRight` (`KismetMathLibrary.ComposeRotators` _output_get_2 (`KismetMathLibrary.MakeRotator` 0.0 0.0 (* (`self.RotateAmount`) -1.0)))))

(event `OpenDoors`
  ;[1 1 1] Open doors
  (set `self.DoorsState` "NewEnumerator3"))

(event `CloseDoors`
  ;[1 1 1] Close doors
  (set `self.DoorsState` "NewEnumerator2"))

(event `self.ReceiveTick`
  (params (DeltaSeconds :type "Float (single-precision)"))
  ;[1 1 1] Interpolate door rotations
  (switch `/Game/Blueprints/Doors/E_DoorState` (`self.DoorsState`)
    (:`NewEnumerator2`
      (`self.InterpDoorRotation` (`self.LeftSideDoor`) (`self.ClosedRotationLeft`) DeltaSeconds)
      (`self.InterpDoorRotation` (`self.RightSideDoor`) (`self.ClosedRotationRight`) DeltaSeconds)
      ;[1 1 1] Check if doors are closed
      (if (and (== (`SceneComponent.K2_GetComponentRotation` (`self.LeftSideDoor`)) (`self.ClosedRotationLeft`) :`ErrorTolerance` 0.01) (== (`SceneComponent.K2_GetComponentRotation` (`self.RightSideDoor`)) (`self.ClosedRotationRight`) :`ErrorTolerance` 0.01))
        (set `self.DoorsState` "NewEnumerator0")))
    (:`NewEnumerator3`
      (`self.InterpDoorRotation` (`self.LeftSideDoor`) (`self.OpenRotationLeft`) DeltaSeconds)
      (`self.InterpDoorRotation` (`self.RightSideDoor`) (`self.OpenRotationRight`) DeltaSeconds)
      ;[1 1 1] Check if doors are open
      (if (and (== (`SceneComponent.K2_GetComponentRotation` (`self.LeftSideDoor`)) (`self.OpenRotationLeft`) :`ErrorTolerance` 0.01) (== (`SceneComponent.K2_GetComponentRotation` (`self.RightSideDoor`)) (`self.OpenRotationRight`) :`ErrorTolerance` 0.01))
        (set `self.DoorsState` "NewEnumerator1")))))

(event `self.ReceiveActorBeginOverlap`
  (params (OtherActor :type "Actor Object Reference"))
  (cast `/Game/Blueprints/Enemies/Abomination/BP_Abomination` OtherActor)
  (`self.OpenDoors`))

(fn `InterpDoorRotation`
  (params (Door :type "SceneComponent Object Reference") (`Target Rotation` :type "Rotator Structure") (DeltaTime :type "Float (single-precision)"))
  (`SceneComponent.K2_SetRelativeRotation` Door (`KismetMathLibrary.RInterpTo` (`SceneComponent.RelativeRotation` Door) `Target Rotation` DeltaTime (`self.RotateSpeed`)) false false))

(fn `UserConstructionScript`)