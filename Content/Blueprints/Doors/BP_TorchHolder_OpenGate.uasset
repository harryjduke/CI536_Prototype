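; BP_TorchHolder_OpenGate is a torch holder that opens a gate when its held item is removed.
; It listens to the Holder component's OnHeldHoldableChanged event and, when the new holdable is invalid, calls OpenDoors on the referenced Door if that is valid.
; A DoorOpened flag makes this a one-time trigger, with no logic to close the gate again.
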(event `self.Holder.OnHeldHoldableChanged`
  (params (NewHoldable :type "Holdable Object Reference"))
  (bind _door (`self.Door`))
  (if (not (`self.DoorOpened`))
    (`/Engine/EditorBlueprintResources/StandardMacros.IsValid` NewHoldable
      (:`Is Not Valid`
        (`/Engine/EditorBlueprintResources/StandardMacros.IsValid` _door
          (:`Is Valid`
            (set `self.DoorOpened` true)
            (`/Game/Blueprints/Doors/BPGate.OpenDoors` _door)))))))

(fn `UserConstructionScript`
  (`parent.UserConstructionScript`))