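; BP_PlayerCharacter is the player character Blueprint, which keeps its MetaHuman body aligned with the capsule and creates the player UI.
; On crouch input, crouch end and BeginPlay, it moves the Root component to the capsule's bottom, using the scaled half-height, so animations stay correct as capsule height changes.
; BeginPlay also creates the PCUI widget and adds it to the viewport.
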(event `EnhancedInput|/Game/ThirdPerson/Input/Actions/IA_Crouch`
  (params (ActionValue :type Boolean) (ElapsedSeconds :type "Float (double-precision)") (TriggeredSeconds :type "Float (double-precision)") (InputAction :type "InputAction Object Reference" :default "/Game/ThirdPerson/Input/Actions/IA_Crouch.IA_Crouch"))
  (bind (_returnvalue_x _returnvalue_y _returnvalue_z) (`KismetMathLibrary.BreakVector` (`SceneComponent.K2_GetComponentLocation` (`self.CapsuleComponent`))))
  ;[1 1 1] Sets the metahuman to the correct height, needs to be done when crouched changes otherwise animations get scuffed.
  (:`Triggered`
    (`SceneComponent.K2_SetWorldLocation` (`self.Root`) (`KismetMathLibrary.MakeVector` _returnvalue_x _returnvalue_y (- _returnvalue_z (`CapsuleComponent.GetScaledCapsuleHalfHeight` (`self.CapsuleComponent`)))) false false :!label _label)))

(event `self.K2_OnEndCrouch`
  (params (HalfHeightAdjust :type "Float (single-precision)") (ScaledHalfHeightAdjust :type "Float (single-precision)"))
  ;[1 1 1] Sets the metahuman to the correct height, needs to be done when crouched changes otherwise animations get scuffed.
  (goto _label))

(event `self.ReceiveBeginPlay`
  (`|ExecutionSequence`
    (:`then_0`
      (goto _label))
    (:`then_1`
      ;[1 1 1] UI
      (bind _returnvalue (`|CreateWidget` "/Game/UI/PCUI.PCUI_C"))
      (`UserWidget.AddToViewport` _returnvalue 0))))

(fn `UserConstructionScript`)