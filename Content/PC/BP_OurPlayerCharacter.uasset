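; Player character Blueprint for a MetaHuman pawn, with a mockup pause toggle, resume and quit events, and the PCUI widget created on play.
; On play, crouch input and crouch end, it moves Root to the capsule's bottom to keep animations aligned.
; That same chain then applies delayed environmental self-damage and prints Health.
; Tick prints horizontal speed for debugging.
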(event `EnhancedInput|/Game/ThirdPerson/Input/Actions/IA_Pause`
  (params (ActionValue :type Boolean) (ElapsedSeconds :type "Float (double-precision)") (TriggeredSeconds :type "Float (double-precision)") (InputAction :type "InputAction Object Reference" :default "/Game/ThirdPerson/Input/Actions/IA_Pause.IA_Pause"))
  ;[1 1 1] Quick pausing mockup
  (:`Completed`
    (`/Engine/EditorBlueprintResources/StandardMacros.FlipFlop`
      (:`A`
        ;;[1 1 1] pausing game
        (set `self.isPaused` true)
        (set `PlayerController.bShowMouseCursor` true (`GameplayStatics.GetPlayerController` 0))
        (`GameplayStatics.SetGamePaused` true))
      (:`B`
        ;;[1 1 1] Unpausing game
        (set `PlayerController.bShowMouseCursor` false (`GameplayStatics.GetPlayerController` 0) :!label _label)
        (set `self.isPaused` false)
        (`GameplayStatics.SetGamePaused` false)))))

(event `self.ReceiveBeginPlay`
  (bind (_returnvalue_x _returnvalue_y _returnvalue_z) (`KismetMathLibrary.BreakVector` (`SceneComponent.K2_GetComponentLocation` (`self.CapsuleComponent`))))
  ;[1 1 1] on play
  (`|ExecutionSequence`
    (:`then_0`
      ;[1 1 1] Sets the metahuman to the correct height, needs to be done when crouched changes otherwise animations get scuffed.
      (`SceneComponent.K2_SetWorldLocation` (`self.Root`) (`KismetMathLibrary.MakeVector` _returnvalue_x _returnvalue_y (- _returnvalue_z (`CapsuleComponent.GetScaledCapsuleHalfHeight` (`self.CapsuleComponent`)))) false false :!label _label_2)
      (`KismetSystemLibrary.Delay` 0.2)
      (`GameplayStatics.ApplyDamage` self 8.0 null null "/Engine/EngineDamageTypes/DmgTypeBP_Environmental.DmgTypeBP_Environmental_C")
      (`KismetSystemLibrary.PrintString` (`KismetStringLibrary.Conv_DoubleToString` (`self.Health`))))
    (:`then_1`
      (bind _returnvalue (`|CreateWidget` "/Game/PC/PCUI.PCUI_C"))
      (`UserWidget.AddToViewport` _returnvalue 0))))

(event `ResumeGame`
  ;[1 1 1] Quick pausing mockup
  ;;[1 1 1] Unpausing game
  (goto _label))

(event `QuitClicked`
  ;[1 1 1] Basic quit code
  (`KismetSystemLibrary.QuitGame` null "Quit"))

(event `self.K2_OnStartCrouch`
  (params (HalfHeightAdjust :type "Float (single-precision)") (ScaledHalfHeightAdjust :type "Float (single-precision)"))
  ;[1 1 1] Sets the metahuman to the correct height, needs to be done when crouched changes otherwise animations get scuffed.
)

(event `EnhancedInput|/Game/ThirdPerson/Input/Actions/IA_Crouch`
  (params (ActionValue :type Boolean) (ElapsedSeconds :type "Float (double-precision)") (TriggeredSeconds :type "Float (double-precision)") (InputAction :type "InputAction Object Reference" :default "/Game/ThirdPerson/Input/Actions/IA_Crouch.IA_Crouch"))
  ;[1 1 1] Sets the metahuman to the correct height, needs to be done when crouched changes otherwise animations get scuffed.
  (:`Triggered`
    (goto _label_2)))

(event `self.K2_OnEndCrouch`
  (params (HalfHeightAdjust :type "Float (single-precision)") (ScaledHalfHeightAdjust :type "Float (single-precision)"))
  ;[1 1 1] Sets the metahuman to the correct height, needs to be done when crouched changes otherwise animations get scuffed.
  (goto _label_2))

(event `self.ReceiveTick`
  (params (DeltaSeconds :type "Float (single-precision)"))
  (`KismetSystemLibrary.PrintString` (`KismetStringLibrary.Concat_StrStr` "current velocity is " (`KismetStringLibrary.Conv_DoubleToString` (`KismetMathLibrary.VSizeXY` (`MovementComponent.Velocity` (`self.CharacterMovement`))))) true true (struct :`G` 0.66 :`B` 1.0 :`A` 1.0) DeltaSeconds))

(fn `UserConstructionScript`)